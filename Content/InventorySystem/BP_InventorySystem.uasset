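; BP_InventorySystem holds a player's item slots and toggles the inventory window.
; On BeginPlay it sizes the slot array, and AddToInventory writes non-stackable items into the first slot matching an empty default struct.
; Stackable items have no handling yet.
; ToggleInventory creates or removes the widget, centered on the ALS controller's HUD canvas, switching between UI-only and game-only input.
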(event `self.ReceiveBeginPlay`
  (`self.PrepareInventory`))

(fn `AddToInventory`
  (params (ContentToAdd :type "/Game/InventorySystem/SlotStructure Structure"))
  (returns (Success :type Boolean))
  (if (not (`.IsStackable_5_6010B4814DA3BA0BDC3622880DD63768` (break `/Game/InventorySystem/ItemStructure` (break `/Game/InventorySystem/SlotStructure` ContentToAdd))))
    (`self.CreateStack` (`local.ContentToAdd`))
    (return true)))

(fn `CreateStack`
  (params (ContentToAdd :type "/Game/InventorySystem/SlotStructure Structure"))
  (bind _inventory (`self.Inventory`))
  (`KismetArrayLibrary.Array_Set` _inventory (`KismetArrayLibrary.Array_Find` _inventory (make `/Game/InventorySystem/SlotStructure` (struct :`Name` "NSLOCTEXT(\"[9D9D15C146E857C05CC70898DCB05603]\", \"2CB8E36F4E8027553485A38BEF7A8380\", \"Null\")" :`IsStackable` true :`Description` "NSLOCTEXT(\"[9D9D15C146E857C05CC70898DCB05603]\", \"4239C24543AE60219F473D8398FB2D31\", \"Null\")" :`IsConsumable` true :`MaxStackSize` 3))) ContentToAdd))

(fn `PrepareInventory`
  (`KismetArrayLibrary.Array_Resize` (`self.Inventory`) (`self.NumberOfSlots`)))

(fn `ToggleInventory`
  (`self.InventoryWindow`
    (:`then`
      (`Widget.RemoveFromParent` (`self.InventoryWindow`))
      (set `self.InventoryWindow` null)
      (`WidgetBlueprintLibrary.SetInputMode_GameOnly` (`GameplayStatics.GetPlayerController` 0)))
    (:`else`
      (bind _returnvalue (`|CreateWidget` "/Game/InventorySystem/InventoryUI/InventoryWindow.InventoryWindow_C" null self))
      (set `self.InventoryWindow` _returnvalue)
      (bind _asals_player_controller (cast `/Game/AdvancedLocomotionV4/Blueprints/CharacterLogic/ALS_Player_Controller` (`GameplayStatics.GetPlayerController` 0)))
      (bind _returnvalue_2 (`CanvasPanel.AddChildToCanvas` (`/Game/InventorySystem/InventoryUI/HUD.HudCanvas` (`/Game/AdvancedLocomotionV4/Blueprints/CharacterLogic/ALS_Player_Controller.HudWidget` _asals_player_controller)) (`self.InventoryWindow`)))
      (`CanvasPanelSlot.SetAutoSize` _returnvalue_2 true)
      (`CanvasPanelSlot.SetAlignment` _returnvalue_2 (0.5 0.5))
      (`CanvasPanelSlot.SetAnchors` _returnvalue_2 (`self.Anchor`))
      (`CanvasPanelSlot.SetPosition` _returnvalue_2 (0.0 0.0))
      (`WidgetBlueprintLibrary.SetInputMode_UIOnlyEx` (`GameplayStatics.GetPlayerController` 0) (`self.InventoryWindow`) "LockAlways"))))