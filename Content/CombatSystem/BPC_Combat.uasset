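; BPC_Combat is a melee combat component handling targeting, light attacks and hit reactions for its owning character.
; EnterCombatMode sphere-scans for opposing combatants, and Tick focuses a close, well-aligned one while idle, showing its widget bar.
; Light attacks rotate toward that focus and play a montage, briefly ignoring root motion when moving.
; While tracing is on, hand-sphere or sword-box traces hit each target once, sending montage-mapped reactions that parrying blocks.
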(event `Trace On`
  (params (AttackType :type "/Game/CombatSystem/E_AttackType Enum" :default "NewEnumerator0") (`Trace?` :type Boolean) (`RightHand?` :type Boolean))
  ;[1 1 1] Trace ACtion
  (bind _output_get (set `self.AttackType` AttackType))
  (switch `/Game/CombatSystem/E_AttackType` _output_get
    (:`NewEnumerator0`
      (set `self.RightHand?` `RightHand?`))
    (:`NewEnumerator1`
      _))
  (if `Trace?`
    (set `self.TraceOn?` true)
    (else
      (set `self.TraceOn?` false)
      (`KismetArrayLibrary.Array_Clear` (`self.EnemyToHit`)))))

(event `self.ReceiveTick`
  (params (DeltaSeconds :type "Float (single-precision)"))
  (`self.FindEnemy`)
  (if (`self.TraceOn?`)
    (`self.PerformTrace`)))

(event `PerformTrace`
  (bind _enemytohit (`self.EnemyToHit`))
  ;[1 1 1] Trace ACtion
  (bind (_outhits _returnvalue) (`self.SelectAttackTrace`))
  (if _returnvalue
    (for _array_element _outhits
      (bind (_bblockinghit _binitialoverlap _time _distance _location _impactpoint _normal _impactnormal _physmat _hitactor) (`GameplayStatics.BreakHitResult` _array_element))
      (`/Engine/EditorBlueprintResources/StandardMacros.IsValid` (`self.GetCombatClass` _hitactor)
        (:`Is Valid`
          (if (not (`KismetArrayLibrary.Array_Contains` _enemytohit _hitactor))
            (`KismetArrayLibrary.Array_Add` _enemytohit _hitactor)
            (`self.GetHit` (`self.GetCombatClass` _hitactor) (`self.GetOwner`) (`BlueprintMapLibrary.Map_Find` (`self.Montages`) (`AnimInstance.GetCurrentActiveMontage` (`self.AnimInstance`))))
            (`GameplayStatics.PlayWorldCameraShake` null (`Actor.K2_GetActorLocation` (`self.GetOwner`)) 0.0 0.0)))))))

(event `Initialize`
  (params (Mesh :type "SkeletalMeshComponent Object Reference") (CharMovement :type "CharacterMovementComponent Object Reference") (Widget :type "WidgetComponent Object Reference") (Sword :type "StaticMeshComponent Object Reference"))
  ;[1 1 1] Begin Play
  (bind _output_get (set `self.Mesh` Mesh))
  (set `self.AnimInstance` (`SkeletalMeshComponent.GetAnimInstance` _output_get))
  (set `self.CharMovement` CharMovement)
  (set `self.WidgetBar` Widget)
  (set `self.Sword` Sword))

(event `Action Input`
  (params (`Attack Move` :type "/Game/CombatSystem/E_AttackMove Enum" :default "NewEnumerator0") (Overlay :type "/Game/AdvancedLocomotionV4/Data/Enums/ALS_OverlayState Enum" :default "NewEnumerator0"))
  ;[1 1 1] Action Input
  (bind _output_get (set `self.StoredKey` `Attack Move`))
  (set `self.Overlay` Overlay)
  (if (not (`self.isAttacking?`))
    (`self.Consumed Key` _output_get)
    (set `self.StoredKey` "NewEnumerator0")))

(event `GetHit`
  (params (Attacker :type "Actor Object Reference") (HitReaction :type "/Game/CombatSystem/HitReaction Structure"))
  ;[1 1 1] Trace ACtion
  (if (not (`self.IsParrying?`))
    (`AnimInstance.Montage_Play` (`self.AnimInstance`) (`.GetHit_4_644AD31341E878B740836498481520ED` (break `/Game/CombatSystem/HitReaction` HitReaction)) 1.0 "MontageLength" 0.0 true)
    (`self.RotateToEnemy` Attacker)))

(event `Consumed Key`
  (params (`Attack Move` :type "/Game/CombatSystem/E_AttackMove Enum" :default "NewEnumerator0"))
  ;[1 1 1] Action Input
  (switch `/Game/CombatSystem/E_AttackMove` `Attack Move`
    (:`NewEnumerator1`
      (`self.LightAttack`))))

(event `ShowBar`
  (params (`Show?` :type Boolean))
  (`SceneComponent.SetVisibility` (`self.WidgetBar`) `Show?` false))

(event `AttachWeapon`
  (params (`Add?` :type Boolean))
  (`SceneComponent.K2_AttachToComponent` (`self.Sword`) (`self.Mesh`) (select `bool` `Add?` :`false` "spine_03Socket" :`true` "hand_rSocket" :!type "Name") "KeepRelative" "KeepRelative" "KeepRelative" true))

(event `SelectFocusEenemy`
  (params (Enemy :type "Actor Object Reference"))
  (`/Engine/EditorBlueprintResources/StandardMacros.IsValid` Enemy
    (:`Is Valid`
      (bind _focusenemy (`self.FocusEnemy`)
        (:`then`
          (`self.ShowBar` (`self.GetCombatClass` _focusenemy) false))
        (:`else`
          _))
      (bind _output_get (set `self.FocusEnemy` Enemy))
      (`self.ShowBar` (`self.GetCombatClass` _output_get) true))
    (:`Is Not Valid`
      (bind _focusenemy_2 (`self.FocusEnemy`)
        (:`then`
          (`self.ShowBar` (`self.GetCombatClass` _focusenemy_2) false))
        (:`else`)))))

(fn `CanAttack?`
  (returns (ReturnValue :type Boolean))
  (return (and (`|EnumEquality` (`self.ActiveState`) "NewEnumerator0") (not (`NavMovementComponent.IsFalling` (`self.CharMovement`))))))

(fn `CheckAutoFind`
  (bind _savectrlrot (`self.SaveCtrlRot`))
  (bind (_returnvalue_roll _returnvalue_pitch _returnvalue_yaw) (`KismetMathLibrary.BreakRotator` (`Controller.GetControlRotation` (`GameplayStatics.GetPlayerController` 0))))
  (bind (_returnvalue_roll_2 _returnvalue_pitch_2 _returnvalue_yaw_2) (`KismetMathLibrary.BreakRotator` (`Controller.GetControlRotation` (`GameplayStatics.GetPlayerController` 0))))
  (if (> (`KismetMathLibrary.VSize` (`PawnMovementComponent.GetLastInputVector` (`self.CharMovement`))) 0.0)
    (`/Engine/EditorBlueprintResources/StandardMacros.DoOnce` false :!label _label
      (:`Completed`
        (set `self.SaveCtrlRot` _returnvalue_yaw_2)
        (set `self.AutoFind?` false)))
    (elif (or (> _returnvalue_yaw (+ _savectrlrot 0.0)) (< _returnvalue_yaw (- _savectrlrot 35.0)))
      (set `self.AutoFind?` true)
      (goto _label :!via `Reset`))))

(fn `EnableRootMotion`
  (`AnimInstance.SetRootMotionMode` (`self.AnimInstance`) "RootMotionFromMontagesOnly"))

(fn `EnterCombatMode`
  (bind _returnvalue (`self.GetOwner`))
  (bind _enemy (`self.Enemy`))
  (bind _returnvalue_2 (`Actor.K2_GetActorLocation` _returnvalue))
  (bind (_outhits _returnvalue_3) (`KismetSystemLibrary.SphereTraceMultiForObjects` _returnvalue_2 _returnvalue_2 1000.0 (`|MakeArray` "ObjectTypeQuery3" :!type "EObjectTypeQuery Enum") false (`|MakeArray` _returnvalue) "ForDuration" true (struct :`R` 1.0 :`A` 1.0) (struct :`G` 1.0 :`A` 1.0) 2.0))
  (if _returnvalue_3
    (set `self.CombatMode?` true)
    (for _array_element _outhits
      (bind (_bblockinghit _binitialoverlap _time _distance _location _impactpoint _normal _impactnormal _physmat _hitactor) (`GameplayStatics.BreakHitResult` _array_element))
      (bind _returnvalue_4 (`self.GetCombatClass` _hitactor))
      (if (and (not (`KismetArrayLibrary.Array_Contains` _enemy _hitactor)) (`KismetSystemLibrary.IsValid` _returnvalue_4) (!= (`/Game/CombatSystem/BPC_Combat.IsEnemy?` _returnvalue_4) (`self.IsEnemy?`)))
        (`KismetArrayLibrary.Array_Add` _enemy _hitactor)))
    (else
      (`KismetArrayLibrary.Array_Clear` (`self.Enemy`))
      (set `self.CombatMode?` false))))

(fn `FindEnemy`
  (locals (TempEnemy :type "Actor Object Reference") (TempDot :type "Float (double-precision)") (TempFoundDot :type "Float (double-precision)") (TempFoundEnemy :type "Actor Object Reference"))
  (bind _returnvalue (`self.GetOwner`))
  (bind _enemy (`self.Enemy`))
  (if (`|EnumEquality` (`self.ActiveState`) "NewEnumerator0")
    (if (> (`KismetArrayLibrary.Array_Length` _enemy) 0)
      (`self.CheckAutoFind`)
      (for _array_element _enemy
        (set `local.TempEnemy` _array_element)
        (if (< (`Actor.GetDistanceTo` _array_element _returnvalue) 600.0)
          (bind _output_get (set `local.TempDot` (`self.CaclulateEnemyLocation` _array_element _returnvalue)))
          (if (> _output_get (`local.TempFoundDot`))
            (set `local.TempFoundDot` (`local.TempDot`))
            (set `local.TempFoundEnemy` (`local.TempEnemy`)))))
      (if (and (> (`local.TempFoundDot`) 0.5) (`KismetSystemLibrary.IsValid` (`local.TempFoundEnemy`)))
        (`self.SelectFocusEenemy` (`local.TempFoundEnemy`))
        (else
          (set `local.TempFoundDot` 0.0)
          (set `local.TempFoundEnemy` null)))
      (else
        (`self.SelectFocusEenemy` null)))))

(fn `GetCombatClass`
  (params (Target :type "Actor Object Reference"))
  (returns (ReturnValue :type "/Game/CombatSystem/BPC_Combat Object Reference"))
  (return (`Actor.GetComponentByClass` Target "BPC_Combat_C")))

(fn `IgnoreRootMotion`
  (if (!= (`PawnMovementComponent.GetLastInputVector` (`self.CharMovement`)) (0.0 0.0 0.0))
    (`AnimInstance.SetRootMotionMode` (`self.AnimInstance`) "IgnoreRootMotion")
    (`KismetSystemLibrary.K2_SetTimer` null "EnableRootMotion" 0.32)))

(fn `LightAttack`
  (if (`self.CanAttack?`)
    (set `self.ActiveState` "NewEnumerator1")
    (`self.IgnoreRootMotion`)
    (`self.RotateToEnemy` (`self.FocusEnemy`))
    (switch `/Game/AdvancedLocomotionV4/Data/Enums/ALS_OverlayState` (`self.Overlay`)
      (:`NewEnumerator0`
        (`AnimInstance.Montage_Play` (`self.AnimInstance`) "/Game/CombatSystem/Greatsword/0__3Combos_Retargeted_For_ALS/GreatSword_Attack_3Combo_1_Montage.GreatSword_Attack_3Combo_1_Montage" 1.0 "MontageLength" 0.0 true))
      (:`NewEnumerator18`
        (`AnimInstance.Montage_Play` (`self.AnimInstance`) "/Game/CombatSystem/Greatsword/0__3Combos_Retargeted_For_ALS/GreatSword_Attack_3Combo_1_Montage.GreatSword_Attack_3Combo_1_Montage" 1.0 "MontageLength" 0.0 true)))))

(fn `SelectAttackTrace`
  (returns (OutHits :type "Array of HitResult Structure") (ReturnValue :type Boolean))
  (bind _sword (`self.Sword`))
  (bind _returnvalue (`SceneComponent.GetSocketLocation` (`self.Mesh`) (select `bool` (`self.RightHand?`) :`false` "middle_01_l" :`true` "middle_01_r" :!type "Name")))
  (switch `/Game/CombatSystem/E_AttackType` (`self.AttackType`)
    (:`NewEnumerator0`
      ;[1 1 1] Null
      (bind (_outhits _returnvalue_2) (`KismetSystemLibrary.SphereTraceMultiForObjects` _returnvalue _returnvalue 20.0 (`|MakeArray` "ObjectTypeQuery3" :!type "EObjectTypeQuery Enum") false (`|MakeArray` (`self.GetOwner`)) "ForOneFrame"))
      (return _outhits _returnvalue_2))
    (:`NewEnumerator1`
      ;[1 1 1] Sword
      (bind (_outhits_2 _returnvalue_3) (`KismetSystemLibrary.BoxTraceMultiForObjects` (`SceneComponent.GetSocketLocation` _sword "Socket1") (`SceneComponent.GetSocketLocation` _sword "Socket2") (10.0 2.0 0.0) (`SceneComponent.GetSocketRotation` _sword "Socket1") (`|MakeArray` "ObjectTypeQuery3" :!type "EObjectTypeQuery Enum") false (`|MakeArray` (`self.GetOwner`)) "ForOneFrame"))
      (return _outhits_2 _returnvalue_3))))