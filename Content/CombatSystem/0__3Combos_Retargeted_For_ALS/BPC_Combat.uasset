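; BPC_Combat is a combat Blueprint component that plays a great sword light attack montage from player action input.
; Initialize caches the mesh, AnimInstance and movement; ActionInput stores the move and consumes it immediately unless already attacking.
; LightAttack sets the active state and resets it on a fixed timer.
; When movement input exists, root motion is briefly ignored, then restored to montage-only by a timer.
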(event `Initialize`
  (params (Mesh :type "SkeletalMeshComponent Object Reference") (CharMovement :type "CharacterMovementComponent Object Reference"))
  (bind _output_get (set `self.Mesh` Mesh))
  (set `self.AnimInstance` (`SkeletalMeshComponent.GetAnimInstance` _output_get))
  (set `self.Char Movement` CharMovement))

(event `Action Input`
  (params (`Attack Move` :type "/Game/CombatSystem/0__3Combos_Retargeted_For_ALS/E_AttackMove Enum" :default "NewEnumerator0"))
  (bind _output_get (set `self.StoredKey` `Attack Move`))
  (if (not (`self.isAttacking?`))
    (`self.Consumed Key` _output_get)
    (set `self.StoredKey` "NewEnumerator0")))

(event `Consumed Key`
  (params (`Attack Move` :type "/Game/CombatSystem/0__3Combos_Retargeted_For_ALS/E_AttackMove Enum" :default "NewEnumerator0"))
  (switch `/Game/CombatSystem/0__3Combos_Retargeted_For_ALS/E_AttackMove` `Attack Move`
    (:`NewEnumerator1`
      (`self.LightAttack`))))

(fn `EnableRootMotion`
  (`AnimInstance.SetRootMotionMode` (`self.AnimInstance`) "RootMotionFromMontagesOnly"))

(fn `IgnoreRootMotion`
  (if (!= (`PawnMovementComponent.GetLastInputVector` (`self.Char Movement`)) (0.0 0.0 0.0))
    (`AnimInstance.SetRootMotionMode` (`self.AnimInstance`) "IgnoreRootMotion")
    (`KismetSystemLibrary.K2_SetTimer` null "EnableRootMotion" 0.32)))

(fn `LightAttack`
  (set `self.ActiveState` "NewEnumerator1")
  (`self.IgnoreRootMotion`)
  (`AnimInstance.Montage_Play` (`self.AnimInstance`) "/Game/CombatSystem/0__3Combos_Retargeted_For_ALS/GreatSword_Attack_3Combo_1_Montage.GreatSword_Attack_3Combo_1_Montage" 1.0 "MontageLength" 0.0 true)
  (`KismetSystemLibrary.K2_SetTimer` null "ResetState" 3.0))

(fn `ResetState`
  (set `self.ActiveState` "NewEnumerator0"))